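; Inventory component that stores the player's items as a map from item to count.
; Add and remove events adjust stacks, drop emptied entries and refresh the inventory widget on FirstPersonCharacter.
; GetItem withdraws up to the requested amount and returns the number taken, while HasItem checks presence.
; UseItem spawns a temporary actor of the item's class, calls Use, consumes one through GetItem and destroys the actor, without checking possession first.
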(event Custom|Add%20Item
  (params (Pickable :type Pickable%20Structure) (Count :type Integer))
  (bind _items (Variables|Default|GetItems))
  (bind (_value _returnvalue) (Utilities|Map|Find _items Pickable))
  ;[1 1 1] Pick Up Item
  (if _returnvalue
    (Utilities|Map|Add _items Pickable (+ _value Count))
    (else
      (Utilities|Map|Add _items Pickable Count)))
  (bind _asfirst_person_character (Utilities|Casting|CastToFirstPersonCharacter (Game|GetPlayerCharacter 0)))
  (Default|RefreshInventory (Variables|/Game/FirstPersonBP/Blueprints/FirstPersonCharacter.FirstPersonCharacter_C|GetInventoryWidgetRef _asfirst_person_character) (Variables|Default|GetItems)))

(event Custom|Remove%20Item
  (params (Item :type Pickable%20Structure) (Count :type Integer))
  (bind _items (Variables|Default|GetItems))
  (bind (_value _returnvalue) (Utilities|Map|Find _items Item))
  (bind _returnvalue_2 (- _value Count))
  ;[1 1 1] Remove Item
  (if _returnvalue
    (if (<= _returnvalue_2 0)
      (Utilities|Map|Remove _items Item)
      (else
        (Utilities|Map|Add _items Item _returnvalue_2)))
    (bind _asfirst_person_character (Utilities|Casting|CastToFirstPersonCharacter (Game|GetPlayerCharacter 0)))
    (Default|RefreshInventory (Variables|/Game/FirstPersonBP/Blueprints/FirstPersonCharacter.FirstPersonCharacter_C|GetInventoryWidgetRef _asfirst_person_character) (Variables|Default|GetItems))
    (else
      (Development|PrintString "Item not foud"))))

(event Custom|UseItem
  (params (Item :type Pickable%20Structure))
  (bind _returnvalue (Game|SpawnActorfromClass (.Class (Utilities|Struct|BreakPickable Item)) (Math|Conversions|ToTransform(Vector) "0, 0, 0") "AdjustIfPossibleButAlwaysSpawn" 0 0))
  (Default|Use _returnvalue)
  (CallFunction|GetItem Item 1)
  (Actor|DestroyActor _returnvalue))

(fn GetItem
  (params (Item :type Pickable%20Structure) (Count :type Integer))
  (bind _items (Variables|Default|GetItems))
  (bind (_value _returnvalue) (Utilities|Map|Find _items Item))
  (if _returnvalue
    (if (<= Count _value)
      (LocalVariables|SetItemsGot Count)
      (else
        (LocalVariables|SetItemsGot _value)))
    (CallFunction|RemoveItem Item (LocalVariables|GetItemsGot))
    (else
      (LocalVariables|SetItemsGot 0)))
  (return (LocalVariables|GetItemsGot)))

(fn HasItem
  (params (Item :type Pickable%20Structure))
  (return (Utilities|Map|Contains (Variables|Default|GetItems) Item)))