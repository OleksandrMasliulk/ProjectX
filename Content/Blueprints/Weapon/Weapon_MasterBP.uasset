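; Master weapon Blueprint that manages ammo and fires a hitscan shot for the first-person player.
; Ammo fills to max on begin play, and Shoot either reloads when empty or spends one round.
; Each shot line-traces on Visibility from player 0's first-person camera along its forward vector, drawing debug lines.
; The trace result is unused, and ammo and reloads are only printed to screen.
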(event Custom|Shoot
  ;[1 1 1] Shoot
  (if (<= (Variables|Default|GetcurrAmmo) 0)
    (CallFunction|Reload)
    (else
      (bind _result (Math|Integer|DecrementInt (Variables|Default|GetcurrAmmo))
        (:%20%20
          (bind _output_get (Variables|Default|SetcurrAmmo _result))
          (Development|PrintString (Utilities|String|ToString(Integer) _output_get))
          (bind _asfirst_person_character (Utilities|Casting|CastToFirstPersonCharacter (Game|GetPlayerCharacter 0)))
          (Collision|LineTraceByChannel (Transformation|GetWorldLocation (Variables|/Game/FirstPersonBP/Blueprints/FirstPersonCharacter.FirstPersonCharacter_C|GetFirstPersonCamera _asfirst_person_character)) (+ (Transformation|GetWorldLocation (Variables|/Game/FirstPersonBP/Blueprints/FirstPersonCharacter.FirstPersonCharacter_C|GetFirstPersonCamera _asfirst_person_character)) (* (Math|Vector|GetForwardVector (Transformation|GetWorldRotation (Variables|/Game/FirstPersonBP/Blueprints/FirstPersonCharacter.FirstPersonCharacter_C|GetFirstPersonCamera _asfirst_person_character))) 5000)) "TraceTypeQuery1" false 0 "ForDuration"))))))

(event Custom|Reload
  ;[1 1 1] Reload
  (Development|PrintString "RELOAD")
  (Variables|Default|SetcurrAmmo (Variables|Default|GetmaxAmmo)))

(event EventBeginPlay
  ;[1 1 1] Init
  (bind _output_get (Variables|Default|SetcurrAmmo (Variables|Default|GetmaxAmmo)))
  (Development|PrintString (Utilities|String|ToString(Integer) _output_get)))