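; AI controller meant to walk an AI through the level's TargetPoint actors one after another.
; Every Tick gathers all TargetPoints and calls AIMoveTo on the one at PointIndex, with no Pawn input supplied.
; Each success passes a DoN capped at the point count to increment PointIndex, with no wrap or reset.
; An unconnected SimpleMoveToLocation toward the first point is left unused.
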(event EventBeginPlay)

(event EventTick
  (params (DeltaSeconds :type Float%20%28single-precision%29))
  (bind _outactors (Actor|GetAllActorsOfClass "/Script/Engine.TargetPoint"))
  (AI|AIMoveTo 0 "0, 0, 0" (Utilities|Array|Get(acopy) _outactors (Variables|Default|GetPoint_Index)) 5.0 false
    (:OnSuccess
      (Utilities|FlowControl|DoN (Utilities|Array|Length _outactors)
        (:Exit
          (bind _result (Math|Integer|IncrementInt (Variables|Default|GetPoint_Index))
            (:%20%20
              (Variables|Default|SetPoint_Index _result))))))))

(fn ConstructionScript)