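; Notebook_BP is an interactible notebook that acts as a save point.
; On Interract it runs the parent interaction, prints a "GAME SAVED" message and calls its Save event.
; Save casts the game mode to FirstPersonGameMode, writes the RespawnPoint's world transform into SaveData as the respawn transform, then calls the game mode's Save.
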(event Custom|Save
  (bind _asfirst_person_game_mode (Utilities|Casting|CastToFirstPersonGameMode (Game|GetGameMode)))
  (Variables|/Game/Blueprints/LevelDataSave.LevelDataSave_C|SetRespawnTransform (Variables|/Game/FirstPersonBP/Blueprints/FirstPersonGameMode.FirstPersonGameMode_C|GetSaveData _asfirst_person_game_mode) (Transformation|GetWorldTransform (Variables|Default|GetRespawnPoint)))
  (Default|Save _asfirst_person_game_mode))

(event EventInterract
  (params (User :type Actor%20Object%20Reference))
  (|CallParentFunction User)
  (Development|PrintString "GAME SAVED")
  (CallFunction|Save))

(fn ConstructionScript
  (|CallParentFunction))