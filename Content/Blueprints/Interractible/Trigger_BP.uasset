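; Trigger volume that starts or completes an objective when the player's FirstPersonCharacter enters its box.
; On begin overlap, boolean flags choose the action for its ObjectiveID, with start taking priority over complete.
; Each action finds the ObjectiveController through GetActorOfClass and calls AddObjective or CompleteObjective on it.
; The trigger has no one-shot guard, so every qualifying overlap repeats the call.
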(event OnComponentBeginOverlap(Box)
  (params (OverlappedComponent :type Primitive%20Component%20Object%20Reference) (OtherActor :type Actor%20Object%20Reference) (OtherComp :type Primitive%20Component%20Object%20Reference) (OtherBodyIndex :type Integer) (bFromSweep :type Boolean) (SweepResult :type Hit%20Result%20Structure%20%28by%20ref%29))
  (bind _objectiveid (Variables|Default|GetobjectiveID))
  (Utilities|Casting|CastToFirstPersonCharacter OtherActor)
  (if (Variables|Default|GetstartObjective?)
    (CallFunction|StartObjective _objectiveid)
    (elif (Variables|Default|GetcompleteObjective?)
      (CallFunction|CompleteObjective _objectiveid))))

(event OnComponentEndOverlap(Box)
  (params (OverlappedComponent :type Primitive%20Component%20Object%20Reference) (OtherActor :type Actor%20Object%20Reference) (OtherComp :type Primitive%20Component%20Object%20Reference) (OtherBodyIndex :type Integer)))

(event EventStartObjective
  (params (id :type Integer))
  (bind _returnvalue (Actor|GetActorOfClass "/Game/Blueprints/Objectives/ObjectiveController.ObjectiveController_C"))
  (Default|AddObjective _returnvalue id))

(event EventCompleteObjective
  (params (id :type Integer))
  (bind _returnvalue (Actor|GetActorOfClass "/Game/Blueprints/Objectives/ObjectiveController.ObjectiveController_C"))
  (Default|CompleteObjective _returnvalue id))

(fn ConstructionScript)