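; Pickable_BP is an interactible world item that the first-person player can pick up into their inventory.
; On BeginPlay it looks up its item row in Pickable_DT by ItemID, destroying itself if none is found.
; On interaction it stops the character's search for interactible objects, adds the item and count to that character's inventory, then destroys itself.
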(event Custom|Pick%20Up
  (params (PlayerInv :type Inventory%20Object%20Reference))
  (Default|AddItem PlayerInv (Variables|Default|GetItem) (Variables|Default|GetCount))
  (Actor|DestroyActor))

(event EventBeginPlay
  (bind _returnvalue (Utilities|GetDataTableRow "/Game/Blueprints/Interractible/Pickable/Pickable_DT.Pickable_DT" (Utilities|String|StringToName (Utilities|String|ToString(Integer) (Variables|Default|GetItemID))))
    (:then
      (Variables|Default|SetItem _returnvalue))
    (:RowNotFound
      (Development|PrintString "No item found")
      (Actor|DestroyActor))))

(event EventInterract
  (params (User :type Actor%20Object%20Reference))
  (bind _asfirst_person_character (Utilities|Casting|CastToFirstPersonCharacter User))
  (Default|StopLookingforInterractibleObject _asfirst_person_character)
  (CallFunction|PickUp (Variables|/Game/FirstPersonBP/Blueprints/FirstPersonCharacter.FirstPersonCharacter_C|GetInventory _asfirst_person_character)))

(fn ConstructionScript
  (|CallParentFunction))