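; Medkit pickable that restores half of the player's maximum health when used.
; The Use event runs the parent logic, prints a debug message, then casts player 0's character to FirstPersonCharacter.
; It writes CurrHealth on the character directly, using a branch to cap the result at MaxHealth.
; BeginPlay is disabled and the construction script only calls its parent.
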(event EventBeginPlay
  (|CallParentFunction) ; This node is disabled and will not be called.\nDrag off pins to build functionality.
)

(event EventUse
  (|CallParentFunction)
  (Development|PrintString "Medkit used")
  (bind _asfirst_person_character (Utilities|Casting|CastToFirstPersonCharacter (Game|GetPlayerCharacter 0)))
  (if (> (+ (Variables|/Game/FirstPersonBP/Blueprints/FirstPersonCharacter.FirstPersonCharacter_C|GetcurrHealth _asfirst_person_character) (/ (Variables|/Game/FirstPersonBP/Blueprints/FirstPersonCharacter.FirstPersonCharacter_C|GetmaxHealth _asfirst_person_character) 2)) (Variables|/Game/FirstPersonBP/Blueprints/FirstPersonCharacter.FirstPersonCharacter_C|GetmaxHealth _asfirst_person_character))
    (Variables|/Game/FirstPersonBP/Blueprints/FirstPersonCharacter.FirstPersonCharacter_C|SetcurrHealth _asfirst_person_character (Variables|/Game/FirstPersonBP/Blueprints/FirstPersonCharacter.FirstPersonCharacter_C|GetmaxHealth _asfirst_person_character))
    (else
      (Variables|/Game/FirstPersonBP/Blueprints/FirstPersonCharacter.FirstPersonCharacter_C|SetcurrHealth _asfirst_person_character (+ (Variables|/Game/FirstPersonBP/Blueprints/FirstPersonCharacter.FirstPersonCharacter_C|GetcurrHealth _asfirst_person_character) (/ (Variables|/Game/FirstPersonBP/Blueprints/FirstPersonCharacter.FirstPersonCharacter_C|GetmaxHealth _asfirst_person_character) 2))))))

(fn ConstructionScript
  (|CallParentFunction))