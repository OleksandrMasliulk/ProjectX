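; Locked door interactable that needs a specific inventory item to unlock before it behaves like its parent.
; Interacting while locked calls Unlock, which looks up ItemNeeded in the Pickable_DT data table and checks the player character's Inventory.
; If the item is present it takes one and clears IsLocked, so later interactions run the parent logic.
; Otherwise it shows the LockedTooltip widget created at BeginPlay.
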(event Custom|Unlock
  (bind _asfirst_person_character (Utilities|Casting|CastToFirstPersonCharacter (Game|GetPlayerCharacter 0)))
  (bind _returnvalue (Utilities|GetDataTableRow "/Game/Blueprints/Interractible/Pickable/Pickable_DT.Pickable_DT" (Utilities|String|StringToName (Utilities|String|ToString(Integer) (Variables|Default|GetitemNeeded))))
    (:then
      (bind _hasitem (Default|HasItem (Variables|/Game/FirstPersonBP/Blueprints/FirstPersonCharacter.FirstPersonCharacter_C|GetInventory _asfirst_person_character) _returnvalue))
      (if _hasitem
        (Default|GetItem (Variables|/Game/FirstPersonBP/Blueprints/FirstPersonCharacter.FirstPersonCharacter_C|GetInventory _asfirst_person_character) _returnvalue 1)
        (Variables|Default|SetisLocked false)
        (else
          (UserInterface|Viewport|AddtoViewport (Variables|Default|GetwidgetRef) 0))))))

(event EventInterract
  (params (User :type Actor%20Object%20Reference))
  (if (Variables|Default|GetisLocked)
    (CallFunction|Unlock)
    (else
      (|CallParentFunction User))))

(event EventBeginPlay
  (bind _returnvalue (UserInterface|CreateWidget "/Game/Blueprints/UI/LockedTooltip.LockedTooltip_C" (Game|GetPlayerController 0)))
  (Variables|Default|SetwidgetRef _returnvalue))

(fn ConstructionScript
  (|CallParentFunction))