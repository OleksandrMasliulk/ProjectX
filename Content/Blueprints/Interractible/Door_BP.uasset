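; Interactable door Blueprint that toggles between open and closed when a user interacts with it.
; Interract runs the parent handler, then branches on IsClosed to call Open or Close and play OpenDoor or DoorClosed.
; Open and Close instantly yaw the Pivot component a quarter turn in opposite directions in world space, without interpolation, and update IsClosed.
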(event Custom|Open
  (bind _pivot (Variables|Default|GetPivot))
  (bind _returnvalue (Transformation|GetWorldRotation _pivot))
  (Transformation|SetWorldRotation _pivot (Math|Rotator|MakeRotator (.roll _returnvalue) (.pitch _returnvalue) (+ (.yaw _returnvalue) 9e+01)) false false)
  (Variables|Default|SetisClosed false))

(event Custom|Close
  (bind _pivot (Variables|Default|GetPivot))
  (bind _returnvalue (Transformation|GetWorldRotation _pivot))
  (Transformation|SetWorldRotation _pivot (Math|Rotator|MakeRotator (.roll _returnvalue) (.pitch _returnvalue) (- (.yaw _returnvalue) 9e+01)) false false)
  (Variables|Default|SetisClosed true))

(event EventInterract
  (params (User :type Actor%20Object%20Reference))
  (|CallParentFunction User)
  (if (Variables|Default|GetisClosed)
    (CallFunction|Open)
    (Audio|Components|Audio|Play (Variables|Default|GetOpen_Door) 0.0)
    (else
      (CallFunction|Close)
      (Audio|Components|Audio|Play (Variables|Default|GetDoor_Closed) 0.0))))

(fn ConstructionScript
  (|CallParentFunction))