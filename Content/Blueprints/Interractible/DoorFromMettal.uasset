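; Interactable metal door Blueprint that the player opens and closes, with an optional locked state.
; Interact shows a widget on screen while the door is locked, otherwise toggles it through Open or Close based on IsClosed.
; Activate clears the lock so later interactions can move the door.
; The construction script only runs the parent's, and Open and Close are not defined in this file.
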(event EventActivate
  (Variables|Default|SetisLocked false))

(event EventInterract
  (params (User :type Actor%20Object%20Reference))
  (if (Variables|Default|GetisLocked)
    (UserInterface|Viewport|AddtoViewport (Variables|Default|GetwidgetRef) 0)
    (elif (Variables|Default|GetisClosed)
      (CallFunction|Open)
      (else
        (CallFunction|Close)))))

(fn ConstructionScript
  (|CallParentFunction))