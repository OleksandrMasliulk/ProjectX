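; Master Blueprint for interactible objects that the first-person character can find and use.
; A Box trigger tells an overlapping FirstPersonCharacter to start looking for interactible objects, and to stop when it leaves.
; The Interract event takes a User and only prints a debug message naming that user and the object.
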(event OnComponentBeginOverlap(Box)
  (params (OverlappedComponent :type Primitive%20Component%20Object%20Reference) (OtherActor :type Actor%20Object%20Reference) (OtherComp :type Primitive%20Component%20Object%20Reference) (OtherBodyIndex :type Integer) (bFromSweep :type Boolean) (SweepResult :type Hit%20Result%20Structure%20%28by%20ref%29))
  (bind _asfirst_person_character (Utilities|Casting|CastToFirstPersonCharacter OtherActor))
  (Default|StartLookingforInterractibleObject _asfirst_person_character))

(event OnComponentEndOverlap(Box)
  (params (OverlappedComponent :type Primitive%20Component%20Object%20Reference) (OtherActor :type Actor%20Object%20Reference) (OtherComp :type Primitive%20Component%20Object%20Reference) (OtherBodyIndex :type Integer))
  (bind _asfirst_person_character (Utilities|Casting|CastToFirstPersonCharacter OtherActor))
  (Default|StopLookingforInterractibleObject _asfirst_person_character))

(event Custom|Interract
  (params (User :type Actor%20Object%20Reference))
  (Development|PrintString (Utilities|String|Append (Utilities|GetObjectName User) " has interracted with " (Utilities|GetObjectName self))))

(fn ConstructionScript)