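; Interactable note actor that shows its text content in a Note widget when the player uses it.
; On BeginPlay it creates the Note widget for the first player controller and caches the reference.
; Interract calls the parent handler, fills the widget with NoteContent, adds it to the viewport, shows the mouse cursor and switches input to UI-only with the widget focused.
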(event EventInterract
  (params (User :type Actor%20Object%20Reference))
  (bind _returnvalue (Game|GetPlayerController 0))
  (bind _notewidgetref (Variables|Default|GetNoteWidgetRef))
  (|CallParentFunction User)
  (Default|SetNoteContent _notewidgetref (Variables|Default|GetNoteContent))
  (UserInterface|Viewport|AddtoViewport _notewidgetref 0)
  (Variables|/Script/Engine.PlayerController|SetbShowMouseCursor _returnvalue true)
  (Input|SetInputModeUIOnly _returnvalue (Variables|Default|GetNoteWidgetRef) "DoNotLock"))

(event EventBeginPlay
  (bind _returnvalue (UserInterface|CreateWidget "/Game/Blueprints/UI/Note.Note_C" (Game|GetPlayerController 0)))
  (Variables|Default|SetNoteWidgetRef _returnvalue))

(fn ConstructionScript
  (|CallParentFunction))