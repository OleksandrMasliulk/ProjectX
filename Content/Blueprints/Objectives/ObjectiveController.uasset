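; ObjectiveController is an actor that tracks objectives and their completion state and shows them on screen.
; On BeginPlay it creates the ObjectivesUI widget, adds it to the viewport and registers the first two objectives.
; AddObjective and CompleteObjective look up ObjectivesDT rows by integer ID converted to a row name, store the row as a map key with a completion bool and update the widget.
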(event Custom|AddObjective
  (params (id :type Integer))
  (bind _returnvalue (Utilities|GetDataTableRow "/Game/Blueprints/Objectives/ObjectivesDT.ObjectivesDT" (Utilities|String|StringToName (Utilities|String|ToString(Integer) id)))
    (:then
      (Utilities|Map|Add (Variables|Default|Getobjectives) _returnvalue false)
      (Default|AddObjective (Variables|Default|GetObjectiives%20UI%20Ref) _returnvalue))))

(event Custom|CompleteObjective
  (params (id :type Integer))
  (bind _returnvalue (Utilities|GetDataTableRow "/Game/Blueprints/Objectives/ObjectivesDT.ObjectivesDT" (Utilities|String|StringToName (Utilities|String|ToString(Integer) id)))
    (:then
      (Utilities|Map|Add (Variables|Default|Getobjectives) _returnvalue true)
      (Default|ObjectiveCompleted (Variables|Default|GetObjectiives%20UI%20Ref) _returnvalue))))

(event EventBeginPlay
  (bind _returnvalue (UserInterface|CreateWidget "/Game/Blueprints/UI/ObjectivesUI.ObjectivesUI_C"))
  (bind _output_get (Variables|Default|SetObjectiives%20UI%20Ref _returnvalue))
  (UserInterface|Viewport|AddtoViewport _output_get 0)
  (for _index (range 0 1)
    (CallFunction|AddObjective _index)))

(fn ConstructionScript)