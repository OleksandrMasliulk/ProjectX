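; Inventory Blueprint that tracks picked-up items and their quantities in an Items map keyed by item.
; AddItem adds the given count to an existing entry or creates a new one.
; RemoveItem takes away one unit, deletes the entry when none remain, and prints a message if the item is missing.
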(event Custom|Add%20Item
  (params (Pickable :type Pickable%20Structure) (Count :type Integer))
  (bind _items (Variables|Default|GetItems))
  (bind (_value _returnvalue) (Utilities|Map|Find _items Pickable))
  ;[1 1 1] Pick Up Item
  (if _returnvalue
    (Utilities|Map|Add _items Pickable (+ _value Count))
    (else
      (Utilities|Map|Add _items Pickable Count))))

(event Custom|Remove%20Item
  (params (Item :type Pickable%20Structure))
  (bind _items (Variables|Default|GetItems))
  (bind (_value _returnvalue) (Utilities|Map|Find _items Item))
  ;[1 1 1] Remove Item
  (if _returnvalue
    (bind _result (Math|Integer|DecrementInt _value)
      (:%20%20
        (if (<= _result 0)
          (Utilities|Map|Remove _items Item)
          (else
            (Utilities|Map|Add _items Item _result)))))
    (else
      (Development|PrintString "Item not foud"))))